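; An unlocked door Blueprint that swings open and closed when interacted with, playing a wooden door sound for each direction.
; BeginPlay caches the mesh's starting rotation, and Interact, gated by CanPressE and CanInteract, toggles the Opened state.
; The TL_Rotate timeline plays from start or reverses to lerp yaw 100 degrees from that rotation.
; A short delay fired from the timeline's update re-enables interaction.
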(event `self.ReceiveBeginPlay`
  (set `self.StartingRotation` (`SceneComponent.RelativeRotation` (`self.StaticMesh`))))

(event `/Game/GameSystems/Traces/BPI_Interaction.Interact`
  (bind (_startingrotation_roll _startingrotation_pitch _startingrotation_yaw) (`KismetMathLibrary.BreakRotator` (`self.StartingRotation`)))
  (bind _staticmesh (`self.StaticMesh`))
  (if (`self.CanPressE`)
    (if (`self.CanInteract`)
      (set `self.CanInteract` false)
      (if (`self.Opened`)
        (set `self.Opened` false)
        (`GameplayStatics.PlaySoundAtLocation` "/Game/SmallSoundKit/SSKCue/DoorsCue/Drs_Wood_Door_Close_01_Cue.Drs_Wood_Door_Close_01_Cue" (`SceneComponent.K2_GetComponentLocation` _staticmesh) (struct) 1.0 1.0 0.0 null null null)
        (bind (_direction _alpha) (`Timeline|TL_Rotate` :!via `Reverse` :!label _label)
          (:`Update`
            (`SceneComponent.K2_SetRelativeRotation` (`self.StaticMesh`) (`KismetMathLibrary.MakeRotator` _startingrotation_roll _startingrotation_pitch (`KismetMathLibrary.Lerp` _startingrotation_yaw (+ _startingrotation_yaw 100.0) _alpha)) false false)
            (`KismetSystemLibrary.Delay` 0.2)
            (set `self.CanInteract` true)))
        (else
          (set `self.Opened` true)
          (`GameplayStatics.PlaySoundAtLocation` "/Game/SmallSoundKit/SSKCue/DoorsCue/Drs_Wood_Door_Open_01_Cue.Drs_Wood_Door_Open_01_Cue" (`SceneComponent.K2_GetComponentLocation` _staticmesh) (struct) 1.0 1.0 0.0 null null null)
          (goto _label :!via `PlayFromStart`))))))

(fn `UserConstructionScript`
  (`parent.UserConstructionScript`))