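; First-person player character with movement, look, sprint, timeline-driven crouch and zoom, and a HUD.
; A looping timer targets a camera sphere trace that notifies BPI_Interaction actors; E interacts with the current one.
; Tick picks camera shakes by movement state, while another timer controls the footstep timeline by speed.
; A downward trace plays footstep sounds by surface type, but its only call sits in an unexecuted timeline branch.
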(event `self.ReceiveBeginPlay`
  (bind _returnvalue (`KismetSystemLibrary.K2_SetTimer` null "Create Interaction Trace" 0.01 true))
  (set `self.Interaction Timer` _returnvalue)
  (bind _returnvalue_2 (`|CreateWidget` "/Game/GameSystems/Hud/UI_HUD.UI_HUD_C"))
  (`UserWidget.AddToViewport` _returnvalue_2 0)
  (`self.Footsteps Timer`))

(event `InputAxis|LookUpDown`
  (params (AxisValue :type "Float (single-precision)"))
  ;[1 1 1] Looking Logic
  (`self.AddControllerPitchInput` AxisValue))

(event `InputAxis|LookRightLeft`
  (params (AxisValue :type "Float (single-precision)"))
  ;[1 1 1] Looking Logic
  (`self.AddControllerYawInput` AxisValue))

(event `Key|E`
  (params (Key :type "Key Structure"))
  ;[1 1 1] Traces
  (:`Pressed`
    (message `/Game/GameSystems/Traces/BPI_Interaction.Interact` (`self.Trace Item`))))

(event `Create Interaction Trace`
  ;[1 1 1] Traces
  (`self.Interaction Trace`))

(event `InputAxis|MoveForwardBackward`
  (params (AxisValue :type "Float (single-precision)"))
  (bind (_returnvalue_roll _returnvalue_pitch _returnvalue_yaw) (`KismetMathLibrary.BreakRotator` (`self.GetControlRotation`)))
  ;[1 1 1] Forward&Backward, Right&Left
  (`self.AddMovementInput` (`KismetMathLibrary.GetForwardVector` (`KismetMathLibrary.MakeRotator` 0.0 0.0 _returnvalue_yaw)) AxisValue))

(event `InputAxis|MoveRightLeft`
  (params (AxisValue :type "Float (single-precision)"))
  (bind (_returnvalue_roll _returnvalue_pitch _returnvalue_yaw) (`KismetMathLibrary.BreakRotator` (`self.GetControlRotation`)))
  ;[1 1 1] Forward&Backward, Right&Left
  (`self.AddMovementInput` (`KismetMathLibrary.GetRightVector` (`KismetMathLibrary.MakeRotator` 0.0 0.0 _returnvalue_yaw)) AxisValue))

(event `InputAction|Crouch`
  (params (Key :type "Key Structure"))
  (bind _charactermovement (`self.CharacterMovement`))
  ;[1 1 1] Crouch
  (:`Pressed`
    (set `CharacterMovementComponent.MaxWalkSpeed` 100.0 _charactermovement)
    (set `self.Crouched` true)
    (bind (_direction _crouchalpha) (`Timeline|Brouch_TL` :!label _label)
      (:`Update`
        (`CapsuleComponent.SetCapsuleHalfHeight` (`self.CapsuleComponent`) (`KismetMathLibrary.Lerp` 88.0 45.0 _crouchalpha) true))))
  (:`Released`
    (set `CharacterMovementComponent.MaxWalkSpeed` 300.0 _charactermovement)
    (set `self.Crouched` false)
    (goto _label :!via `Reverse`)))

(event `InputAction|Sprint`
  (params (Key :type "Key Structure"))
  (bind _charactermovement (`self.CharacterMovement`))
  (bind _crouched (`self.Crouched`))
  ;[1 1 1] Sprint
  (:`Pressed`
    (if (not _crouched)
      (set `CharacterMovementComponent.MaxWalkSpeed` 450.0 _charactermovement)))
  (:`Released`
    (if (not _crouched)
      (set `CharacterMovementComponent.MaxWalkSpeed` 300.0 _charactermovement))))

(event `Footsteps Timer`
  ;[1 1 1] Footsteps sound
  (`KismetSystemLibrary.K2_SetTimerDelegate` (delegate `CheckForFootstep`) 0.01 true))

(event `Headbob`
  (bind _returnvalue (`GameplayStatics.GetPlayerController` 0))
  (bind _returnvalue_2 (`KismetMathLibrary.VSize` (`self.GetVelocity`)))
  ;[1 1 1] Handbob
  (if (and (> _returnvalue_2 0.0) (`self.CanJump`))
    (if (<= (`CharacterMovementComponent.MaxWalkSpeed` (`self.CharacterMovement`)) 100.0)
      (`PlayerController.ClientStartCameraShake` :`self` _returnvalue :`Shake` "/Game/PlayerCharacter/Headbob/Crouch.Crouch_C")
      (elif (<= _returnvalue_2 300.0)
        (`PlayerController.ClientStartCameraShake` :`self` _returnvalue :`Shake` "/Game/PlayerCharacter/Headbob/Walk.Walk_C")
        (else
          (`PlayerController.ClientStartCameraShake` :`self` _returnvalue :`Shake` "/Game/PlayerCharacter/Headbob/Sprint.Sprint_C"))))
    (else
      (`PlayerController.ClientStartCameraShake` :`self` _returnvalue :`Shake` "/Game/PlayerCharacter/Headbob/Idle.Idle_C"))))

(event `CheckForFootstep`
  (bind _footstep_tl (`self.Footstep_TL`))
  (bind _footstep_tl_2 (`self.Footstep_TL`))
  ;[1 1 1] Footsteps sound
  (if (> (`KismetMathLibrary.VSizeXY` (`MovementComponent.Velocity` (`self.CharacterMovement`))) 0.0)
    (`/Engine/EditorBlueprintResources/StandardMacros.CompareFloat` (`CharacterMovementComponent.MaxWalkSpeed` (`self.CharacterMovement`)) 300.0
      (:`>`
        (`TimelineComponent.SetPlayRate` _footstep_tl_2 1.5)
        (`TimelineComponent.Play` _footstep_tl_2))
      (:`==`
        (`TimelineComponent.SetPlayRate` _footstep_tl_2 1.0)
        (`TimelineComponent.Play` _footstep_tl_2))
      (:`<`
        (`TimelineComponent.Stop` _footstep_tl)))
    (else
      (`TimelineComponent.Stop` _footstep_tl))))

(event `self.ReceiveTick`
  (params (DeltaSeconds :type "Float (single-precision)"))
  ;[1 1 1] Handbob
  (`self.Headbob`))

(event `InputAction|Zoom`
  (params (Key :type "Key Structure"))
  (:`Pressed`
    (bind (_direction _zoom) (`Timeline|Timeline_0` :!label _label_2)
      (:`Update`
        (`CameraComponent.SetFieldOfView` (`self.Camera`) (`KismetMathLibrary.Lerp` 90.0 55.0 _zoom)))))
  (:`Released`
    (goto _label_2 :!via `Reverse`)))

(fn `FootStepsTrace`
  (bind _returnvalue (`self.K2_GetActorLocation`))
  (bind _his_result_location (`self.His Result Location`))
  (if (not (`self.AfterFootStepsCoolDown`))
    (bind (_outhit _returnvalue_2) (`KismetSystemLibrary.SphereTraceSingle` _returnvalue (`KismetMathLibrary.MakeVector` (.x _returnvalue) (.y _returnvalue) (- (.z _returnvalue) (`CapsuleComponent.GetScaledCapsuleHalfHeight` (`self.CapsuleComponent`)))) (`CapsuleComponent.GetScaledCapsuleRadius` (`self.CapsuleComponent`)) "TraceTypeQuery1"))
    (if _returnvalue_2
      (set `self.His Result Location` (`.Location` (`GameplayStatics.BreakHitResult` _outhit)))
      (switch `EPhysicalSurface` (`GameplayStatics.GetSurfaceType` _outhit)
        (:`SurfaceType1`
          (`GameplayStatics.PlaySoundAtLocation` "/Game/GameSystems/Footsteps/Sound/ConcreteFS.ConcreteFS" _his_result_location (struct) 1.0 1.0 0.0 null null null null))
        (:`SurfaceType2`
          (`GameplayStatics.PlaySoundAtLocation` "/Game/GameSystems/Footsteps/Sound/WoodFS.WoodFS" _his_result_location (struct) 1.0 1.0 0.0 null null null null))
        (:`SurfaceType3`
          (`GameplayStatics.PlaySoundAtLocation` "/Game/GameSystems/Footsteps/Sound/GrassFS.GrassFS" _his_result_location (struct) 1.0 1.0 0.0 null null null null))
        (:`SurfaceType4`
          (`GameplayStatics.PlaySoundAtLocation` "/Game/GameSystems/Footsteps/Sound/SnowFS.SnowFS" _his_result_location (struct) 1.0 1.0 0.0 null null null null))))))

(fn `Interaction Trace`
  (bind _camera (`self.Camera`))
  (bind _returnvalue (`SceneComponent.K2_GetComponentLocation` _camera))
  (bind _outhit (`KismetSystemLibrary.SphereTraceSingle` _returnvalue (+ _returnvalue (* (`KismetMathLibrary.GetForwardVector` (`SceneComponent.K2_GetComponentRotation` _camera)) 1000.0)) 3.0 "TraceTypeQuery1"))
  (bind (_bblockinghit _binitialoverlap _time _distance _location _impactpoint _normal _impactnormal _physmat _hitactor) (`GameplayStatics.BreakHitResult` _outhit))
  (if (`KismetSystemLibrary.DoesImplementInterface` _hitactor "/Game/GameSystems/Traces/BPI_Interaction.BPI_Interaction_C")
    (if (!= _hitactor (`self.Trace Item`))
      (bind _output_get (set `self.Trace Item` _hitactor))
      (message `/Game/GameSystems/Traces/BPI_Interaction.Can Receive Trace` _output_get true))
    (else
      (message `/Game/GameSystems/Traces/BPI_Interaction.Can Receive Trace` (`self.Trace Item`) false)
      (set `self.Trace Item` null))))

(fn `UserConstructionScript`)